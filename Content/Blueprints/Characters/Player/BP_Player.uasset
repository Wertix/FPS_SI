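; Player character Blueprint built on the Gameplay Ability System, adding weapon, UI and an immunity toggle to its parent class.
; On BeginPlay it runs the parent logic, attaches the weapon through WeaponComponent and shows WBP_SimpleUI, passing it the player's Ability System Component.
; The G key alternates between applying GE_Immune to itself and removing it through the stored effect handle.
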(event `self.ReceiveBeginPlay`
  (`parent.ReceiveBeginPlay`)
  (`SIWeaponComponentBase.AttachWeapon` (`self.WeaponComponent`) self)
  (bind _returnvalue (`|CreateWidget` "/Game/UI/WBP_SimpleUI.WBP_SimpleUI_C" (`GameplayStatics.GetPlayerController` 0) (`AbilitySystemBlueprintLibrary.GetAbilitySystemComponent` self)))
  (`UserWidget.AddToViewport` _returnvalue 0))

(event `Key|G`
  (params (Key :type "Key Structure"))
  (bind _returnvalue (`AbilitySystemBlueprintLibrary.GetAbilitySystemComponent` self))
  (:`Pressed`
    (`/Engine/EditorBlueprintResources/StandardMacros.FlipFlop`
      (:`A`
        (bind _returnvalue_2 (`AbilitySystemComponent.BP_ApplyGameplayEffectToSelf` :`self` _returnvalue :`GameplayEffectClass` "/Game/Blueprints/Abilities/Player/Defensive/GE_Immune.GE_Immune_C"))
        (set `self.GEHandle` _returnvalue_2))
      (:`B`
        (`AbilitySystemComponent.RemoveActiveGameplayEffect` _returnvalue (`self.GEHandle`) -1)))))

(fn `UserConstructionScript`)