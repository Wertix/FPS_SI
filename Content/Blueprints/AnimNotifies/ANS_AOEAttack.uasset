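; Anim notify state for an area attack that detects the characters hit during its animation window.
; Each tick it sphere-traces for pawns between two mesh sockets, ignoring the owner and characters already hit.
; Each new hit sends the owner an ApplyPerformedAbilityEffects gameplay event carrying the target data and effect context, leaving effect application to GAS.
; The hit list clears on notify begin, so each window hits a character only once.
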(fn `Received_NotifyBegin`
  (params (MeshComp :type "SkeletalMeshComponent Object Reference") (Animation :type "AnimSequenceBase Object Reference") (TotalDuration :type "Float (single-precision)") (EventReference :type "AnimNotifyEventReference Structure (by ref)"))
  (returns (ReturnValue :type Boolean))
  (`KismetArrayLibrary.Array_Clear` (`self.HitCharacters`))
  (return true))

(fn `Received_NotifyTick`
  (params (MeshComp :type "SkeletalMeshComponent Object Reference") (Animation :type "AnimSequenceBase Object Reference") (FrameDeltaTime :type "Float (single-precision)") (EventReference :type "AnimNotifyEventReference Structure (by ref)"))
  (returns (ReturnValue :type Boolean))
  (bind _assicharacter_base (cast `SICharacterBase` (`ActorComponent.GetOwner` MeshComp) :!pure true))
  (bind (_outhits _returnvalue) (`KismetSystemLibrary.SphereTraceMultiForObjects` MeshComp (`SceneComponent.GetSocketLocation` MeshComp (`self.TraceSocketStart`)) (`SceneComponent.GetSocketLocation` MeshComp (`self.TraceSocketEnd`)) 10.0 (`|MakeArray` "ObjectTypeQuery3" :!type "EObjectTypeQuery Enum")))
  (if _returnvalue
    (for _array_element _outhits
      (bind _assicharacter_base_2 (cast `SICharacterBase` (`.HitActor` (`GameplayStatics.BreakHitResult` _array_element))))
      (if (and (not (`KismetArrayLibrary.Array_Contains` (`self.HitCharacters`) _assicharacter_base_2)) (!= _assicharacter_base_2 _assicharacter_base))
        (`KismetArrayLibrary.Array_AddUnique` (`self.HitCharacters`) _assicharacter_base_2)
        (`AbilitySystemBlueprintLibrary.SendGameplayEventToActor` _assicharacter_base (struct :`TagName` "Animation.ApplyPerformedAbilityEffects") (make `GameplayEventData` (struct) _assicharacter_base _assicharacter_base_2 null null (`AbilitySystemComponent.MakeEffectContext` (`AbilitySystemBlueprintLibrary.GetAbilitySystemComponent` _assicharacter_base)) (struct) (struct) 0.0 (`AbilitySystemBlueprintLibrary.AbilityTargetDataFromActor` _assicharacter_base_2)))))
    (return true)
    (else
      (return false))))